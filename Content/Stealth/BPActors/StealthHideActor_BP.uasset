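; Stealth hide area actor that marks whatever enters it as hidden, noted as a way to conceal dead bodies.
; Its box overlap sends a "Hidden" or "UnHidden" interface message to the other actor on enter and exit, printing a tag for debug on entry.
; An older, deprecated approach that toggled enemy AI sight perception with a crouch-check loop remains disconnected and never runs.
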(event `self.Box_HideStealthArea.OnComponentBeginOverlap`
  (params (OverlappedComponent :type "PrimitiveComponent Object Reference") (OtherActor :type "Actor Object Reference") (OtherComp :type "PrimitiveComponent Object Reference") (OtherBodyIndex :type Integer) (bFromSweep :type Boolean) (SweepResult :type "HitResult Structure (by ref)"))
  ;[1 1 1] Setting tag for dead bodies to hide them in hide actor
  (message `/Game/Stealth/ThirdPersonBP/Blueprints/ICallToEnemy.IHiddenUnhiddenTag` OtherActor "Hidden")
  (`KismetSystemLibrary.PrintString` (`KismetStringLibrary.Conv_NameToString` (`|GetArrayItem` (`Actor.Tags` OtherActor) 1))))

(event `self.Box_HideStealthArea.OnComponentEndOverlap`
  (params (OverlappedComponent :type "PrimitiveComponent Object Reference") (OtherActor :type "Actor Object Reference") (OtherComp :type "PrimitiveComponent Object Reference") (OtherBodyIndex :type Integer))
  ;[1 1 1] Setting tag for dead bodies to hide them in hide actor
  (message `/Game/Stealth/ThirdPersonBP/Blueprints/ICallToEnemy.IHiddenUnhiddenTag` OtherActor "UnHidden"))

(fn `UserConstructionScript`)