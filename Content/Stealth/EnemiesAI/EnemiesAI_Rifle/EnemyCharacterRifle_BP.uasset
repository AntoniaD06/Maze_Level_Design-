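; Rifle enemy character for the stealth game, handling takedowns, body dragging and alert display.
; AI messages drive the vision cone colour, alert bar and melee montage; melee overlap only prints damage.
; Front and back boxes register it as the player's kill target or warn its controller, with optional shielded-enemy blocking.
; Takedown tags it Dead, unpossesses it and enables dragging, with a trace-based drop; cone rotation and old patrol logic are inactive.
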(event `/Game/Stealth/EnemiesAI/IAI_Interface.ICapsuleRotation`
  (params (CapsuleRotation :type "Rotator Structure"))
  ;[1 1 1] Perception COne Jugaar Deprecated But Perception cone rotates using this technique (Deprecated)
  ;;[1 1 1] Get COne Rotaion from behavior tree
  (bind _output_get (set `self.Capsule Rotation` CapsuleRotation))
  (`KismetSystemLibrary.PrintString` (`KismetStringLibrary.Conv_RotatorToString` _output_get) true true (struct :`R` 1.0 :`B` 0.03671 :`A` 1.0)))

(event `self.ReceiveBeginPlay`
  ;[1 1 1] Event Begin Play
  (`/Game/Stealth/ThirdPersonBP/Blueprints/ThirdPersonCharacter.Event_StealthKillOverlap` (cast `/Game/Stealth/ThirdPersonBP/Blueprints/ThirdPersonCharacter` (`GameplayStatics.GetPlayerCharacter` 0) :!pure true) self)
  (bind _outactors (`GameplayStatics.GetAllActorsOfClass` "/Game/Stealth/BPActors/StealthHideActor_BP.StealthHideActor_BP_C"))
  (for (_array_element _array_index) _outactors
    (`KismetArrayLibrary.Array_Set` (`self.HideActor_Ref`) _array_index _array_element true)))

(event `/Game/Stealth/EnemiesAI/IAI_Interface.PawnObject`
  (params (PawnObject :type "Pawn Object Reference") (`StartRotation?` :type Boolean))
  ;[1 1 1] Perception COne Jugaar Deprecated But Perception cone rotates using this technique (Deprecated)
  ;;[1 1 1] Get Information from AI controller whether to start Perception cone rotation or not
  (set `self.Start Rotation?` `StartRotation?`)
  (`KismetSystemLibrary.PrintString` (`KismetSystemLibrary.GetDisplayName` PawnObject) true true (struct :`G` 0.045145 :`B` 1.0 :`A` 1.0))
  (if (`self.Start Rotation?`)
    (`self.EventStartConeRotation`)
    (else
      (`self.Event_StopConeRotation`))))

(event `Event_StopPerceptionRotation`
  ;[1 1 1] Perception COne Jugaar Deprecated But Perception cone rotates using this technique (Deprecated)
  ;;[1 1 1] Get Information from AI controller whether to start Perception cone rotation or not
)

(event `/Game/Stealth/EnemiesAI/EnemiesAI_Rifle/ICombatRifle_Interface.IVisionConeColour_Rifle`
  (params (ConeColour :type String))
  ;[1 1 1] Vision Cone Colours w.r.t Alert Stats
  (`KismetSystemLibrary.PrintString` ConeColour true true (struct :`R` 0.115642 :`B` 1.0 :`A` 1.0))
  (switch `string` ConeColour
    (:`Green`
      (`PrimitiveComponent.SetMaterial` (`self.StaticMesh_VisionCone`) 0 "/Game/Stealth/Materials/Cone_Green_Inst.Cone_Green_Inst")
      ;;[1 1 1] This is not Shield enemy this is Rifle enemy. SO "is this shielded enemy" public bool will be false always. If you want to make it same difficult as shielded enemy then check true this bool
      (if (`self.IsThisSHieldedEnemy?`)
        (set `self.BlockBackStealthkill?` false)))
    (:`Yellow`
      (`PrimitiveComponent.SetMaterial` (`self.StaticMesh_VisionCone`) 0 "/Game/Stealth/Materials/Cone_Yellow_Inst.Cone_Yellow_Inst")
      (if (`self.IsThisSHieldedEnemy?`) :!label _label
        (set `self.BlockBackStealthkill?` true)))
    (:`Orange`
      (`PrimitiveComponent.SetMaterial` (`self.StaticMesh_VisionCone`) 0 "/Game/Stealth/Materials/Cone_Orange_Inst.Cone_Orange_Inst")
      (goto _label))
    (:`Red`
      (`PrimitiveComponent.SetMaterial` (`self.StaticMesh_VisionCone`) 0 "/Game/Stealth/Materials/Cone_Red_Inst.Cone_Red_Inst")
      (goto _label))))

(event `EventStartConeRotation`
  ;[1 1 1] Perception COne Jugaar Deprecated But Perception cone rotates using this technique (Deprecated)
  ;;[1 1 1] Perception COne Rotation COde
)

(event `Event_StopConeRotation`
  ;[1 1 1] Perception COne Jugaar Deprecated But Perception cone rotates using this technique (Deprecated)
  ;;[1 1 1] Perception COne Rotation COde
)

(event `/Game/Stealth/EnemiesAI/EnemiesAI_Rifle/ICombatRifle_Interface.IMeleeAttackRifle_Function`
  ;[1 1 1] Melee Attack
  (`|PlayMontage` (`self.Mesh`) "/Game/Stealth/EnemiesAnims/Attack_PrimaryA_Montage.Attack_PrimaryA_Montage"
    (:`then`
      (`KismetSystemLibrary.PrintString` "melee attack"))))

(event `Event_AlertStatus`
  (params (AlertBarFloat :type "Float (double-precision)"))
  ;[1 1 1] Updating AlertBar Widget Value
  (bind _aswidget_alert_status (cast `/Game/Stealth/ThirdPersonBP/Blueprints/Widget_AlertStatus` (`WidgetComponent.GetWidget` (`self.Widget_AlertBar`))))
  (`ProgressBar.SetPercent` (`/Game/Stealth/ThirdPersonBP/Blueprints/Widget_AlertStatus.AlertBar` _aswidget_alert_status) AlertBarFloat))

(event `self.Box_MeleeAttackDamage.OnComponentBeginOverlap`
  (params (OverlappedComponent :type "PrimitiveComponent Object Reference") (OtherActor :type "Actor Object Reference") (OtherComp :type "PrimitiveComponent Object Reference") (OtherBodyIndex :type Integer) (bFromSweep :type Boolean) (SweepResult :type "HitResult Structure (by ref)"))
  ;[1 1 1] Melee Attack
  (cast `/Game/Stealth/ThirdPersonBP/Blueprints/ThirdPersonCharacter` OtherActor)
  (`/Engine/EditorBlueprintResources/StandardMacros.DoOnce` false :!label _label_2
    (:`Completed`
      (`KismetSystemLibrary.PrintString` "DamageApplied" true true (struct :`R` 1.0 :`G` 0.144344 :`A` 1.0))
      (`KismetSystemLibrary.Delay` 1.5)
      (goto _label_2 :!via `Reset`))))

(event `self.Box_Back.OnComponentBeginOverlap`
  (params (OverlappedComponent :type "PrimitiveComponent Object Reference") (OtherActor :type "Actor Object Reference") (OtherComp :type "PrimitiveComponent Object Reference") (OtherBodyIndex :type Integer) (bFromSweep :type Boolean) (SweepResult :type "HitResult Structure (by ref)"))
  ;[1 1 1] Overlap box on back of enemy to get stealth kill From Back (Box_Back Collision
  (bind _asthird_person_character (cast `/Game/Stealth/ThirdPersonBP/Blueprints/ThirdPersonCharacter` OtherActor))
  (if (`self.BlockBackStealthkill?`)
    ;[1 1 1] Our Player gets too close to enemy from back (At the moment Will work only if "IsThisShieldedEnemy"  bool set to true
    (message `/Game/Stealth/EnemiesAI/EnemiesAI_Rifle/IEnemyRifleToAI_Interface.IEnemyTooClose` (`self.GetController`))
    (else
      (`/Game/Stealth/ThirdPersonBP/Blueprints/ThirdPersonCharacter.Event_TargetEnemyReference` _asthird_person_character "/Game/Stealth/EnemiesAI/EnemiesAI_Knife/EnemyCharacterKnife_BP.EnemyCharacterKnife_BP_C" self)
      (bind _output_get (set `/Game/Stealth/ThirdPersonBP/Blueprints/ThirdPersonCharacter.InBackStealthKillBox?` true _asthird_person_character))
      (set `self.LocalInBackStealthKillBox?` _output_get)
      (`KismetSystemLibrary.PrintString` "entered"))))

(event `self.Box_Back.OnComponentEndOverlap`
  (params (OverlappedComponent :type "PrimitiveComponent Object Reference") (OtherActor :type "Actor Object Reference") (OtherComp :type "PrimitiveComponent Object Reference") (OtherBodyIndex :type Integer))
  ;[1 1 1] Overlap box on back of enemy to get stealth kill From Back (Box_Back Collision
  ;;[1 1 1] End Overlap
  (bind _asthird_person_character (cast `/Game/Stealth/ThirdPersonBP/Blueprints/ThirdPersonCharacter` OtherActor))
  (set `/Game/Stealth/ThirdPersonBP/Blueprints/ThirdPersonCharacter.InBackStealthKillBox?` false _asthird_person_character)
  (`KismetSystemLibrary.PrintString` "Exit Overlap")
  (set `self.LocalInBackStealthKillBox?` false))

(event `/Game/Stealth/ThirdPersonBP/Blueprints/ICallToEnemy.ICheckInBackStealthKillBox?`
  ;[1 1 1] Overlap box on back of enemy to get stealth kill From Back (Box_Back Collision
  ;;[1 1 1] COnfirmation. Is in back stealth kill box?
  (bind _asthird_person_character (cast `/Game/Stealth/ThirdPersonBP/Blueprints/ThirdPersonCharacter` (`GameplayStatics.GetPlayerCharacter` 0)))
  (`/Game/Stealth/ThirdPersonBP/Blueprints/ThirdPersonCharacter.Event_BackStealthKillBox?` _asthird_person_character (`self.LocalInBackStealthKillBox?`)))

(event `/Game/Stealth/ThirdPersonBP/Blueprints/ICallToEnemy.IDragBody`
  (params (`DesiredEnemy ` :type "Character Object Reference") (DragCOllisionBox :type "SceneComponent Object Reference") (`InStealthKillBox?` :type Boolean))
  ;[1 1 1] Body Drag only when in Box Front back collision boxes after killing enemy
  (if (`self.CanDrag?`)
    (`PrimitiveComponent.SetCollisionEnabled` (`self.CapsuleComponent`) "NoCollision")
    (`self.K2_AttachToComponent` `DesiredEnemy ` DragCOllisionBox "None" "SnapToTarget" "KeepWorld" "KeepWorld" true)
    (else
      (`KismetSystemLibrary.PrintString` "InBox"))))

(event `self.Box_Front.OnComponentBeginOverlap`
  (params (OverlappedComponent :type "PrimitiveComponent Object Reference") (OtherActor :type "Actor Object Reference") (OtherComp :type "PrimitiveComponent Object Reference") (OtherBodyIndex :type Integer) (bFromSweep :type Boolean) (SweepResult :type "HitResult Structure (by ref)"))
  ;[1 1 1] Enemy too close to our character (Box_Front Collision)
  (bind _asthird_person_character (cast `/Game/Stealth/ThirdPersonBP/Blueprints/ThirdPersonCharacter` OtherActor))
  (message `/Game/Stealth/EnemiesAI/EnemiesAI_Rifle/IEnemyRifleToAI_Interface.IEnemyTooClose` (`self.GetController`))
  (if (not (`self.IsThisSHieldedEnemy?`))
    (set `/Game/Stealth/ThirdPersonBP/Blueprints/ThirdPersonCharacter.InFrontKillBox?` true _asthird_person_character)
    (`/Game/Stealth/ThirdPersonBP/Blueprints/ThirdPersonCharacter.Event_TargetEnemyReference` _asthird_person_character "/Game/Stealth/EnemiesAI/EnemiesAI_Knife/EnemyCharacterKnife_BP.EnemyCharacterKnife_BP_C" self)))

(event `/Game/Stealth/ThirdPersonBP/Blueprints/ICallToEnemy.IDragBodyDrop`
  (params (BodyToDrop :type "Character Object Reference"))
  (bind _returnvalue (`self.K2_GetActorLocation` (`GameplayStatics.GetPlayerCharacter` 0)))
  ;[1 1 1] Dropping lifted body. Detaching
  (if (`self.CanDrag?`)
    (bind _outhit (`KismetSystemLibrary.LineTraceSingle` _returnvalue (+ _returnvalue (0.0 0.0 -500.0)) "TraceTypeQuery1" false (`self.HideActor_Ref`) "Persistent"))
    (`self.K2_SetActorLocation` BodyToDrop (+ (`.ImpactPoint` (`GameplayStatics.BreakHitResult` _outhit)) (0.0 0.0 100.0)) true false)
    (`self.K2_DetachFromActor` BodyToDrop "KeepWorld" "KeepWorld" "KeepWorld")
    (`KismetSystemLibrary.Delay` 0.5)
    (`PrimitiveComponent.SetCollisionEnabled` (`self.CapsuleComponent`) "QueryOnly")
    (`PrimitiveComponent.SetCollisionEnabled` (`self.Mesh`) "QueryOnly")
    (else
      (`KismetSystemLibrary.PrintString` "Cant Drag Body Bcoz Enemy is alive"))))

(event `self.Box_Front.OnComponentEndOverlap`
  (params (OverlappedComponent :type "PrimitiveComponent Object Reference") (OtherActor :type "Actor Object Reference") (OtherComp :type "PrimitiveComponent Object Reference") (OtherBodyIndex :type Integer))
  ;[1 1 1] Enemy too close to our character (Box_Front Collision)
  (bind _asthird_person_character (cast `/Game/Stealth/ThirdPersonBP/Blueprints/ThirdPersonCharacter` OtherActor))
  (set `/Game/Stealth/ThirdPersonBP/Blueprints/ThirdPersonCharacter.InFrontKillBox?` false _asthird_person_character))

(event `Event_GetStealthAttack`
  (params (KillBool :type Boolean))
  ;[1 1 1] Stealth Attacll Anim
  (bind _output_get (set `self.BackStealthKill_Anim` KillBool)))

(event `/Game/Stealth/ThirdPersonBP/Blueprints/IAnimations_Interface.IEnemyDeathEnd_Anim`
  ;[1 1 1] Enabling Enemy collision at end of death animation to get hit result from sphere trace
  (`PrimitiveComponent.SetCollisionEnabled` (`self.CapsuleComponent`) "QueryOnly")
  (`PrimitiveComponent.SetCollisionEnabled` (`self.Mesh`) "QueryOnly"))

(event `/Game/Stealth/ThirdPersonBP/Blueprints/ICallToEnemy.IHiddenUnhiddenTag`
  (params (Tag :type Name))
  ;[1 1 1] Enemy Hidden Unhidden Tag at index 1
  (`KismetArrayLibrary.Array_Set` (`self.Tags`) 1 Tag true))

(event `/Game/Stealth/ThirdPersonBP/Blueprints/ICallToEnemy.IDesiredEnemyToTakedown`
  (params (`FrontKillAnimPlay?` :type Boolean))
  (bind _returnvalue (`self.GetController`))
  ;[1 1 1] Stealth Kill animation run and disabling movement - Enemy Death
  (`KismetSystemLibrary.PrintString` (`KismetStringLibrary.Conv_BoolToString` `FrontKillAnimPlay?`) true true (struct :`R` 1.0 :`G` 0.082829 :`A` 1.0))
  (if `FrontKillAnimPlay?`
    (set `self.Front Kill Anim Play?` `FrontKillAnimPlay?`) ; For animation
    (else
      (set `self.BackStealthKill_Anim` true) ; For animation
    ))
  (`CharacterMovementComponent.DisableMovement` (`self.CharacterMovement`))
  (`KismetArrayLibrary.Array_Set` (`self.Tags`) 0 "Dead" true) ; dead tag at index 0 bcoz hidden/unhidden is on 1
  (`ActorComponent.K2_DestroyComponent` (`self.StaticMesh_VisionCone`))
  (`ActorComponent.K2_DestroyComponent` (`self.Widget_AlertBar`))
  (set `self.BlockBackStealthkill?` false) ; For shielded enemy
  (message `/Game/Stealth/EnemiesAI/EnemiesAI_Rifle/IEnemyRifleToAI_Interface.IEnemyRifle_ControllerDeath` _returnvalue)
  (`Controller.UnPossess` _returnvalue)
  (set `self.CanDrag?` true) ; Enemy is killed now you can drag him
)

(fn `UserConstructionScript`)