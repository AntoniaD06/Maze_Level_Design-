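; Pedestrian enemy AI pawn for a stealth game, currently reduced to debug output with its behavior disconnected.
; BeginPlay and Tick print the distance between the movement component's owner and itself, also used as print duration.
; The See Pawn event is empty.
; Unreachable nodes hold a looping target-point patrol using AI MoveTo, a speed change for player sighting and a stealth-kill overlap call to the player character.
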(event `self.ReceiveTick`
  (params (DeltaSeconds :type "Float (single-precision)"))
  (bind _returnvalue (`self.GetDistanceTo` (`PawnMovementComponent.GetPawnOwner` (`self.FloatingPawnMovement`)) self))
  ;[1 1 1] Enemy_AI petrolling
  (`KismetSystemLibrary.PrintText` (`KismetTextLibrary.Conv_DoubleToText` _returnvalue "HalfToEven") true true (struct :`G` 0.66 :`B` 1.0 :`A` 1.0) _returnvalue :!label _label))

(event `self.ReceiveBeginPlay`
  ;[1 1 1] Enemy_AI petrolling
  (goto _label))

(event `self.PawnSensing.OnSeePawn`
  (params (Pawn :type "Pawn Object Reference")))

(fn `UserConstructionScript`)